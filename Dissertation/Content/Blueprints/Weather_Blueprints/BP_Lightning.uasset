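; BP_Lightning is a weather actor that produces a lightning strike with sound and a flash when rain is signaled.
; On BeginPlay it sets the Lightning component's Emissive material parameter to zero and binds LightningStrike to the Raining dispatcher of BP_Weather.
; Each strike waits a short random delay, plays LightningSound, then runs the Strike timeline, whose StrikeTrack drives Emissive to create the flash.
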(event Custom|LightningStrike
  (Utilities|FlowControl|Delay (Math|Random|RandomFloatinRange 0.0 1e+01))
  (Audio|Components|Audio|Play (Variables|Default|GetLightningSound) 0.0)
  (bind _striketrack (Timeline|Strike PlayFromStart)
    (:Update
      (Rendering|Material|SetScalarParameterValueonMaterials (Variables|Default|GetLightning) "Emissive" _striketrack))))

(event EventBeginPlay
  (Rendering|Material|SetScalarParameterValueonMaterials (Variables|Default|GetLightning) "Emissive" 0.0)
  (bind _outactors (Actor|GetAllActorsOfClass "/Game/Blueprints/Weather_Blueprints/BP_Weather.BP_Weather_C"))
  (EventDispatchers|BindEventtoDispatcherRaining _outactors (delegate Custom|LightningStrike)))

(fn ConstructionScript)