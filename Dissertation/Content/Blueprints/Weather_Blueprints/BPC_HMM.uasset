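; Weather component that picks the next weather state using Markov-style transition chances between normal, rain, snow and drought.
; Each Tick it finds BP_Weather and binds WeatherChange to that actor's dispatcher.
; On that event it branches on the actor's current status and stores the result in its own WeatherStatus.
; Each range check rolls a new random number, so effective odds differ from the written ranges and the state can stay unchanged.
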(event Custom|WeatherChange
  (bind _returnvalue (Math|Random|RandomInteger 100))
  (bind _returnvalue_2 (Math|Random|RandomInteger 100))
  (bind _returnvalue_3 (Math|Random|RandomInteger 100))
  (bind _returnvalue_4 (Math|Random|RandomInteger 100))
  (Variables|Default|SetWeatherStatus (Variables|/Game/Blueprints/Weather_Blueprints/BP_Weather.BP_Weather_C|GetWeatherStatus (stale EventTick _returnvalue)))
  ;[1 1 1] Normal transition chances
  (if (Utilities|Enum|Equal(Enum) (Variables|/Game/Blueprints/Weather_Blueprints/BP_Weather.BP_Weather_C|GetWeatherStatus (stale EventTick _returnvalue)) "NewEnumerator0")
    (if (Math|Integer|InRange(Integer) _returnvalue 0 40)
      (Variables|Default|SetWeatherStatus "NewEnumerator0")
      (elif (Math|Integer|InRange(Integer) _returnvalue 41 80)
        (Variables|Default|SetWeatherStatus "NewEnumerator1")
        (elif (Math|Integer|InRange(Integer) _returnvalue 81 100)
          (Variables|Default|SetWeatherStatus "NewEnumerator3"))))
    (else
      ;[1 1 1] Raining transition chances
      (if (Utilities|Enum|Equal(Enum) (Variables|/Game/Blueprints/Weather_Blueprints/BP_Weather.BP_Weather_C|GetWeatherStatus (stale EventTick _returnvalue)) "NewEnumerator1")
        (if (Math|Integer|InRange(Integer) _returnvalue_3 0 50)
          (Variables|Default|SetWeatherStatus "NewEnumerator1")
          (elif (Math|Integer|InRange(Integer) _returnvalue_3 51 84)
            (Variables|Default|SetWeatherStatus "NewEnumerator0")
            (elif (Math|Integer|InRange(Integer) _returnvalue_3 85 100)
              (Variables|Default|SetWeatherStatus "NewEnumerator2"))))
        (else
          ;[1 1 1] Snowing transition chances
          (if (Utilities|Enum|Equal(Enum) (Variables|/Game/Blueprints/Weather_Blueprints/BP_Weather.BP_Weather_C|GetWeatherStatus (stale EventTick _returnvalue)) "NewEnumerator2")
            (if (Math|Integer|InRange(Integer) _returnvalue_4 0 50)
              (Variables|Default|SetWeatherStatus "NewEnumerator2")
              (elif (Math|Integer|InRange(Integer) _returnvalue_4 51 100)
                (Variables|Default|SetWeatherStatus "NewEnumerator3")))
            (else
              ;[1 1 1] Draught transition chances
              (if (Utilities|Enum|Equal(Enum) (Variables|/Game/Blueprints/Weather_Blueprints/BP_Weather.BP_Weather_C|GetWeatherStatus (stale EventTick _returnvalue)) "NewEnumerator3")
                (if (Math|Integer|InRange(Integer) _returnvalue_2 0 70)
                  (Variables|Default|SetWeatherStatus "NewEnumerator3")
                  (elif (Math|Integer|InRange(Integer) _returnvalue_2 71 80)
                    (Variables|Default|SetWeatherStatus "NewEnumerator1")
                    (elif (Math|Integer|InRange(Integer) _returnvalue_2 81 100)
                      (Variables|Default|SetWeatherStatus "NewEnumerator0"))))))))))))

(event EventBeginPlay)

(event EventTick
  (params (DeltaSeconds :type Float%20%28single-precision%29))
  (bind _returnvalue (Actor|GetActorOfClass "/Game/Blueprints/Weather_Blueprints/BP_Weather.BP_Weather_C"))
  (EventDispatchers|BindEventtoDispatcherWeatherChange _returnvalue (delegate Custom|WeatherChange)))