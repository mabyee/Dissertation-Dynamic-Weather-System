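; BP_HMM picks the next weather state (normal, raining, snowing or drought) using a Markov-chain style transition table.
; On BeginPlay it reads the current state from Instance_WeatherStatus and binds WeatherChange to a dispatcher on BP_Weather.
; Each change rolls a random percentage against weighted thresholds for the current state.
; Tick copies the local state back into the Game Instance every frame.
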(event Custom|WeatherChange
  ;[1 1 1] Randomise weather state on key press "F"
  (Variables|Default|SetWeatherStatus (Variables|/Game/Blueprints/Instance_WeatherStatus.Instance_WeatherStatus_C|GetWeatherStatus (stale EventBeginPlay _asinstance_weather_status)))
  (Variables|Default|SetPercent (Math|Random|RandomInteger 100))
  ;[1 1 1] Normal transition chances
  (if (Utilities|Enum|Equal(Enum) (Variables|/Game/Blueprints/Instance_WeatherStatus.Instance_WeatherStatus_C|GetWeatherStatus (stale EventBeginPlay _asinstance_weather_status)) "NewEnumerator0")
    (if (Math|Integer|InRange(Integer) (Variables|Default|GetPercent) 0 40)
      (Variables|Default|SetWeatherStatus "NewEnumerator0")
      (elif (Math|Integer|InRange(Integer) (Variables|Default|GetPercent) 41 80)
        (Variables|Default|SetWeatherStatus "NewEnumerator1")
        (elif (Math|Integer|InRange(Integer) (Variables|Default|GetPercent) 81 100)
          (Variables|Default|SetWeatherStatus "NewEnumerator3"))))
    (else
      ;[1 1 1] Raining transition chances
      (if (Utilities|Enum|Equal(Enum) (Variables|/Game/Blueprints/Instance_WeatherStatus.Instance_WeatherStatus_C|GetWeatherStatus (stale EventBeginPlay _asinstance_weather_status)) "NewEnumerator1")
        (if (Math|Integer|InRange(Integer) (Variables|Default|GetPercent) 0 50)
          (Variables|Default|SetWeatherStatus "NewEnumerator1")
          (elif (Math|Integer|InRange(Integer) (Variables|Default|GetPercent) 51 84)
            (Variables|Default|SetWeatherStatus "NewEnumerator0")
            (elif (Math|Integer|InRange(Integer) (Variables|Default|GetPercent) 85 100)
              (Variables|Default|SetWeatherStatus "NewEnumerator2"))))
        (else
          ;[1 1 1] Snowing transition chances
          (if (Utilities|Enum|Equal(Enum) (Variables|/Game/Blueprints/Instance_WeatherStatus.Instance_WeatherStatus_C|GetWeatherStatus (stale EventBeginPlay _asinstance_weather_status)) "NewEnumerator2")
            (if (Math|Integer|InRange(Integer) (Variables|Default|GetPercent) 0 50)
              (Variables|Default|SetWeatherStatus "NewEnumerator2")
              (elif (Math|Integer|InRange(Integer) (Variables|Default|GetPercent) 51 100)
                (Variables|Default|SetWeatherStatus "NewEnumerator3")))
            (else
              ;[1 1 1] Draught transition chances
              (if (Utilities|Enum|Equal(Enum) (Variables|/Game/Blueprints/Instance_WeatherStatus.Instance_WeatherStatus_C|GetWeatherStatus (stale EventBeginPlay _asinstance_weather_status)) "NewEnumerator3")
                (if (Math|Integer|InRange(Integer) (Variables|Default|GetPercent) 0 70)
                  (Variables|Default|SetWeatherStatus "NewEnumerator3")
                  (elif (Math|Integer|InRange(Integer) (Variables|Default|GetPercent) 71 80)
                    (Variables|Default|SetWeatherStatus "NewEnumerator1")
                    (elif (Math|Integer|InRange(Integer) (Variables|Default|GetPercent) 81 100)
                      (Variables|Default|SetWeatherStatus "NewEnumerator0"))))))))))))

(event EventTick
  (params (DeltaSeconds :type Float%20%28single-precision%29))
  ;[1 1 1] Set global variable from local variable
  (bind _asinstance_weather_status (Utilities|Casting|CastToInstance_WeatherStatus (Game|GetGameInstance)))
  (Variables|/Game/Blueprints/Instance_WeatherStatus.Instance_WeatherStatus_C|SetWeatherStatus _asinstance_weather_status (Variables|Default|GetWeatherStatus)))

(event EventBeginPlay
  ;[1 1 1] Bind event dispatcher to local event and set the first weather status
  (bind _asinstance_weather_status (Utilities|Casting|CastToInstance_WeatherStatus (Game|GetGameInstance)))
  (Variables|Default|SetWeatherStatus (Variables|/Game/Blueprints/Instance_WeatherStatus.Instance_WeatherStatus_C|GetWeatherStatus _asinstance_weather_status))
  (bind _returnvalue (Actor|GetActorOfClass "/Game/Blueprints/Weather_Blueprints/BP_Weather.BP_Weather_C"))
  (EventDispatchers|BindEventtoDispatcherWeatherChange _returnvalue (delegate Custom|WeatherChange)))

(fn ConstructionScript)