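; Weather actor that crossfades rain and snow particle effects according to a randomly chosen WeatherStatus.
; The status is picked on BeginPlay and re-rolled every 30 seconds, with Delays in Tick throttling both the re-roll and the 0.2-second update.
; Normal and Raining drain snow before building rain, while Snowing and Draught do the reverse.
; The clamped amounts drive float parameters on PSRain and PSSnow.
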(event EventBeginPlay
  (Variables|Default|SetWeatherStatus (Utilities|Enum|ByteToEnumEnum_WeatherStatus (Math|Conversions|ToByte(Integer) (Math|Random|RandomIntegerinRange 0 (|GetNumEnumEntries))))))

(event EventTick
  (params (DeltaSeconds :type Float%20%28single-precision%29))
  (bind _increment (Variables|Default|GetIncrement))
  (Utilities|FlowControl|Sequence
    (:then_0
      (Utilities|FlowControl|Delay 0.2)
      (switch Utilities|FlowControl|Switch|SwitchonEnum_WeatherStatus (Variables|Default|GetWeatherStatus)
        (:NewEnumerator0
          (if (<= (Variables|Default|GetSnowAmount) 0.0) :!label _label
            (Variables|Default|SetRainAmount (Math|Float|Clamp(Float) (+ (Variables|Default|GetRainAmount) _increment) 0.0 5e+03))
            (Effects|Components|ParticleSystem|SetFloatParameter (Variables|Default|GetPS_Rain) "RainAmount" (Variables|Default|GetRainAmount) :!label _label_2)
            (else
              (Variables|Default|SetSnowAmount (- (Variables|Default|GetSnowAmount) _increment))
              (Effects|Components|ParticleSystem|SetFloatParameter (Variables|Default|GetPS_Snow) "SnowAmount" (Variables|Default|GetSnowAmount) :!label _label_3))))
        (:NewEnumerator1
          (goto _label))
        (:NewEnumerator2
          (if (<= (Variables|Default|GetRainAmount) 0.0) :!label _label_4
            (Variables|Default|SetSnowAmount (Math|Float|Clamp(Float) (+ (Variables|Default|GetSnowAmount) _increment) 0.0 5e+03))
            (goto _label_3)
            (else
              (Variables|Default|SetRainAmount (- (Variables|Default|GetRainAmount) _increment))
              (goto _label_2))))
        (:NewEnumerator3
          (goto _label_4))))
    (:then_1
      (Utilities|FlowControl|Delay 3e+01)
      (Variables|Default|SetWeatherStatus (Utilities|Enum|ByteToEnumEnum_WeatherStatus (Math|Conversions|ToByte(Integer) (Math|Random|RandomIntegerinRange 0 (|GetNumEnumEntries))))))))

(fn ConstructionScript)