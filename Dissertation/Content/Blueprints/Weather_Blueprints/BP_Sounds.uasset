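; BP_Sounds crossfades rain and snow ambient audio in response to weather changes from BP_Weather.
; On every Tick it looks up BP_Weather and binds to its Raining, Normal, Draught and Snowing dispatchers.
; Each event plays a timeline that lerps volume multipliers from stored amounts, saving the result on finish.
; Normal and Draught fade both sounds out, Snowing swaps rain for snow, and Raining only raises rain.
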(event Custom|Normal
  (bind _newtrack_0 (Timeline|Timeline_1 PlayFromStart)
    (:Update
      (Audio|Components|Audio|SetVolumeMultiplier (Variables|Default|Getrain) (Math|Float|Lerp (Variables|Default|GetrainAmount) 0.0 _newtrack_0) :!class /Script/Engine.AudioComponent)
      (Audio|Components|Audio|SetVolumeMultiplier (Variables|Default|Getsnow) (Math|Float|Lerp (Variables|Default|GetsnowAmount) 0.0 _newtrack_0) :!class /Script/Engine.AudioComponent))
    (:Finished
      (Variables|Default|SetrainAmount (Math|Float|Lerp (Variables|Default|GetrainAmount) 0.0 _newtrack_0))
      (Variables|Default|SetsnowAmount (Math|Float|Lerp (Variables|Default|GetsnowAmount) 0.0 _newtrack_0)))))

(event Custom|Raining
  (bind _newtrack_0 (Timeline|timeline_rain PlayFromStart)
    (:Update
      (Audio|Components|Audio|SetVolumeMultiplier (Variables|Default|Getrain) (Math|Float|Lerp (Variables|Default|GetrainAmount) 1.0 _newtrack_0) :!class /Script/Engine.AudioComponent))
    (:Finished
      (Variables|Default|SetrainAmount (Math|Float|Lerp (Variables|Default|GetrainAmount) 1.0 _newtrack_0)))))

(event Custom|Snowing
  (bind _newtrack_0 (Timeline|timeline_snow PlayFromStart)
    (:Update
      (Audio|Components|Audio|SetVolumeMultiplier (Variables|Default|Getrain) (Math|Float|Lerp (Variables|Default|GetrainAmount) 0.0 _newtrack_0) :!class /Script/Engine.AudioComponent)
      (Audio|Components|Audio|SetVolumeMultiplier (Variables|Default|Getsnow) (Math|Float|Lerp (Variables|Default|GetsnowAmount) 1.0 _newtrack_0) :!class /Script/Engine.AudioComponent))
    (:Finished
      (Variables|Default|SetrainAmount (Math|Float|Lerp (Variables|Default|GetrainAmount) 0.0 _newtrack_0))
      (Variables|Default|SetsnowAmount (Math|Float|Lerp (Variables|Default|GetsnowAmount) 1.0 _newtrack_0)))))

(event Custom|Draught
  (bind _newtrack_0 (Timeline|Timeline_0 PlayFromStart)
    (:Update
      (Audio|Components|Audio|SetVolumeMultiplier (Variables|Default|Getrain) (Math|Float|Lerp (Variables|Default|GetrainAmount) 0.0 _newtrack_0) :!class /Script/Engine.AudioComponent)
      (Audio|Components|Audio|SetVolumeMultiplier (Variables|Default|Getsnow) (Math|Float|Lerp (Variables|Default|GetsnowAmount) 0.0 _newtrack_0) :!class /Script/Engine.AudioComponent))
    (:Finished
      (Variables|Default|SetrainAmount (Math|Float|Lerp (Variables|Default|GetrainAmount) 0.0 _newtrack_0))
      (Variables|Default|SetsnowAmount (Math|Float|Lerp (Variables|Default|GetsnowAmount) 0.0 _newtrack_0)))))

(event EventTick
  (params (DeltaSeconds :type Float%20%28single-precision%29))
  (bind _returnvalue (Actor|GetActorOfClass "/Game/Blueprints/Weather_Blueprints/BP_Weather.BP_Weather_C"))
  (EventDispatchers|BindEventtoDispatcherRaining _returnvalue (delegate Custom|Raining))
  (EventDispatchers|BindEventtoDispatcherNormal _returnvalue (delegate Custom|Normal))
  (EventDispatchers|BindEventtoDispatcherDraught _returnvalue (delegate Custom|Draught))
  (EventDispatchers|BindEventtoDispatcherSnowing _returnvalue (delegate Custom|Snowing)))

(fn ConstructionScript)