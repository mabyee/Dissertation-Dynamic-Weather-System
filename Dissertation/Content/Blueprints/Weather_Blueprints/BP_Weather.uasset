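; Weather controller that picks a random Normal, Raining, Snowing or Draught state at BeginPlay and periodically afterwards.
; Delayed Tick logic runs the active state's event, gradually ramping rain and snow particles, with each waiting for the other to fade before building up.
; States drive puddle and ground snow through MPC_Weather and set wind strength in PN_WindParameters.
; DoOnce gates, reset on each weather roll, limit state-change dispatcher calls.
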(event Custom|Normal
  (params (Normal :type String))
  (bind _increment (Variables|Default|GetIncrement))
  ;[1 1 1] Normal
  (Development|PrintString Normal)
  (if (and (Variables|Default|GetHasSnowStopped) (Variables|Default|GetHasRainStopped))
    _
    (else
      (bind _output_get (Variables|Default|SetRainAmount (- (Variables|Default|GetRainAmount) _increment)))
      (Effects|Components|ParticleSystem|SetFloatParameter (Variables|Default|GetPS_Rain) "RainAmount" _output_get)
      (bind _output_get_2 (Variables|Default|SetSnowAmount (- (Variables|Default|GetSnowAmount) _increment)))
      (Effects|Components|ParticleSystem|SetFloatParameter (Variables|Default|GetPS_Snow) "SnowAmount" _output_get_2)
      (bind _output_get_3 (Variables|Default|SetPuddle_WaterAmount (Math|Float|Clamp(Float) (- (Variables|Default|GetPuddle_WaterAmount) 0.2) 0.0 2e+01)))
      (Rendering|Material|SetScalarParameterValue "/Game/Materials/MPC_Weather.MPC_Weather" "WaterAmount" _output_get_3 :!class /Script/Engine.KismetMaterialLibrary)
      (bind _output_get_4 (Variables|Default|SetFloor_SnowAmount (Math|Float|Clamp(Float) (- (Variables|Default|GetFloor_SnowAmount) 0.2) 0.0 2e+01)))
      (Rendering|Material|SetScalarParameterValue "/Game/Materials/MPC_Weather.MPC_Weather" "SnowAmount" _output_get_4 :!class /Script/Engine.KismetMaterialLibrary)))
  (Utilities|FlowControl|DoOnce false
    (:Completed
      (Default|CallDispatcherNormal)
      (Rendering|Material|SetScalarParameterValue "/Game/PN_interactiveSpruceForest/Materials/PN_WindParameters.PN_WindParameters" "WindStrength" 1.0 :!class /Script/Engine.KismetMaterialLibrary))))

(event Custom|Raining
  (params (Raining :type String))
  (bind _increment (Variables|Default|GetIncrement))
  ;[1 1 1] Raining
  (Development|PrintString Raining)
  (if (Variables|Default|GetHasSnowStopped)
    (Variables|Default|SetPuddle_WaterAmount (Math|Float|Clamp(Float) (+ (Variables|Default|GetPuddle_WaterAmount) 0.1) 0.0 2e+01))
    (Variables|Default|SetFloor_SnowAmount (Math|Float|Clamp(Float) (- (Variables|Default|GetFloor_SnowAmount) 0.2) 0.0 2e+01))
    (bind _output_get (Variables|Default|SetRainAmount (Math|Float|Clamp(Float) (+ (Variables|Default|GetRainAmount) _increment) 0.0 5e+03)))
    (Effects|Components|ParticleSystem|SetFloatParameter (Variables|Default|GetPS_Rain) "RainAmount" _output_get)
    (Rendering|Material|SetScalarParameterValue "/Game/Materials/MPC_Weather.MPC_Weather" "WaterAmount" (Variables|Default|GetPuddle_WaterAmount) :!class /Script/Engine.KismetMaterialLibrary)
    (Rendering|Material|SetScalarParameterValue "/Game/Materials/MPC_Weather.MPC_Weather" "SnowAmount" (Variables|Default|GetFloor_SnowAmount) :!class /Script/Engine.KismetMaterialLibrary)
    (Rendering|Material|SetScalarParameterValue "/Game/Materials/MPC_Weather.MPC_Weather" "SnowOrRain" 1.0 :!class /Script/Engine.KismetMaterialLibrary)
    (Utilities|FlowControl|DoOnce false
      (:Completed
        (Default|CallDispatcherRaining)))
    (else
      (bind _output_get_2 (Variables|Default|SetSnowAmount (- (Variables|Default|GetSnowAmount) _increment)))
      (Effects|Components|ParticleSystem|SetFloatParameter (Variables|Default|GetPS_Snow) "RainAmount" _output_get_2)
      (Rendering|Material|SetScalarParameterValue "/Game/Materials/MPC_Weather.MPC_Weather" "WaterAmount" (Variables|Default|GetPuddle_WaterAmount) :!class /Script/Engine.KismetMaterialLibrary)
      (Rendering|Material|SetScalarParameterValue "/Game/Materials/MPC_Weather.MPC_Weather" "SnowAmount" (Variables|Default|GetFloor_SnowAmount) :!class /Script/Engine.KismetMaterialLibrary)
      (Rendering|Material|SetScalarParameterValue "/Game/Materials/MPC_Weather.MPC_Weather" "SnowOrRain" 1.0 :!class /Script/Engine.KismetMaterialLibrary)))
  (Rendering|Material|SetScalarParameterValue "/Game/PN_interactiveSpruceForest/Materials/PN_WindParameters.PN_WindParameters" "WindStrength" 3.0 :!class /Script/Engine.KismetMaterialLibrary))

(event Custom|Snowing
  (params (Snowing :type String))
  (bind _increment (Variables|Default|GetIncrement))
  ;[1 1 1] Snowing
  (Development|PrintString Snowing)
  (if (Variables|Default|GetHasRainStopped)
    (Variables|Default|SetPuddle_WaterAmount (Math|Float|Clamp(Float) (- (Variables|Default|GetPuddle_WaterAmount) 0.2) 0.0 2e+01))
    (Variables|Default|SetFloor_SnowAmount (Math|Float|Clamp(Float) (+ (Variables|Default|GetFloor_SnowAmount) 0.1) 0.0 2e+01))
    (bind _output_get (Variables|Default|SetSnowAmount (Math|Float|Clamp(Float) (+ (Variables|Default|GetSnowAmount) _increment) 0.0 5e+03)))
    (Effects|Components|ParticleSystem|SetFloatParameter (Variables|Default|GetPS_Snow) "SnowAmount" _output_get)
    (Rendering|Material|SetScalarParameterValue "/Game/Materials/MPC_Weather.MPC_Weather" "WaterAmount" (Variables|Default|GetPuddle_WaterAmount) :!class /Script/Engine.KismetMaterialLibrary)
    (Rendering|Material|SetScalarParameterValue "/Game/Materials/MPC_Weather.MPC_Weather" "SnowAmount" (Variables|Default|GetFloor_SnowAmount) :!class /Script/Engine.KismetMaterialLibrary)
    (Rendering|Material|SetScalarParameterValue "/Game/Materials/MPC_Weather.MPC_Weather" "SnowOrRain" 0.0 :!class /Script/Engine.KismetMaterialLibrary)
    (Utilities|FlowControl|DoOnce false
      (:Completed
        (Default|CallDispatcherSnowing)))
    (else
      (bind _output_get_2 (Variables|Default|SetRainAmount (- (Variables|Default|GetRainAmount) _increment)))
      (Effects|Components|ParticleSystem|SetFloatParameter (Variables|Default|GetPS_Rain) "RainAmount" _output_get_2)
      (Rendering|Material|SetScalarParameterValue "/Game/Materials/MPC_Weather.MPC_Weather" "WaterAmount" (Variables|Default|GetPuddle_WaterAmount) :!class /Script/Engine.KismetMaterialLibrary)
      (Rendering|Material|SetScalarParameterValue "/Game/Materials/MPC_Weather.MPC_Weather" "SnowAmount" (Variables|Default|GetFloor_SnowAmount) :!class /Script/Engine.KismetMaterialLibrary)
      (Rendering|Material|SetScalarParameterValue "/Game/Materials/MPC_Weather.MPC_Weather" "SnowOrRain" 1.0 :!class /Script/Engine.KismetMaterialLibrary)))
  (Rendering|Material|SetScalarParameterValue "/Game/PN_interactiveSpruceForest/Materials/PN_WindParameters.PN_WindParameters" "WindStrength" 2.0 :!class /Script/Engine.KismetMaterialLibrary))

(event Custom|Draught
  (params (Draught :type String))
  (bind _increment (Variables|Default|GetIncrement))
  ;[1 1 1] Draught
  (Development|PrintString Draught)
  (if (and (Variables|Default|GetHasSnowStopped) (Variables|Default|GetHasRainStopped))
    _
    (else
      (bind _output_get (Variables|Default|SetRainAmount (- (Variables|Default|GetRainAmount) _increment)))
      (Effects|Components|ParticleSystem|SetFloatParameter (Variables|Default|GetPS_Rain) "RainAmount" _output_get)
      (bind _output_get_2 (Variables|Default|SetSnowAmount (- (Variables|Default|GetSnowAmount) _increment)))
      (Effects|Components|ParticleSystem|SetFloatParameter (Variables|Default|GetPS_Snow) "SnowAmount" _output_get_2)
      (bind _output_get_3 (Variables|Default|SetPuddle_WaterAmount (Math|Float|Clamp(Float) (- (Variables|Default|GetPuddle_WaterAmount) 0.2) 0.0 2e+01)))
      (Rendering|Material|SetScalarParameterValue "/Game/Materials/MPC_Weather.MPC_Weather" "WaterAmount" _output_get_3 :!class /Script/Engine.KismetMaterialLibrary)
      (bind _output_get_4 (Variables|Default|SetFloor_SnowAmount (Math|Float|Clamp(Float) (- (Variables|Default|GetFloor_SnowAmount) 0.2) 0.0 2e+01)))
      (Rendering|Material|SetScalarParameterValue "/Game/Materials/MPC_Weather.MPC_Weather" "SnowAmount" _output_get_4 :!class /Script/Engine.KismetMaterialLibrary)))
  (Utilities|FlowControl|DoOnce false
    (:Completed
      (Default|CallDispatcherDraught)
      (Rendering|Material|SetScalarParameterValue "/Game/PN_interactiveSpruceForest/Materials/PN_WindParameters.PN_WindParameters" "WindStrength" 0.5 :!class /Script/Engine.KismetMaterialLibrary))))

(event EventBeginPlay
  ;[1 1 1] Setting the weather and initiating the event
  (Variables|Default|SetWeatherStatus (Utilities|Enum|ByteToEnumEnum_WeatherStatus (Math|Conversions|ToByte(Integer) (Math|Random|RandomIntegerinRange 0 (- (|GetNumEnumEntries) 1)))))
  (Utilities|FlowControl|Sequence
    (:then_0
      (Utilities|FlowControl|DoOnce false) ; enters at Reset
    )
    (:then_1
      ;[1 1 1] Normal
      (Utilities|FlowControl|DoOnce false) ; enters at Reset
    )
    (:then_2
      (Utilities|FlowControl|DoOnce false) ; enters at Reset
    )
    (:then_3
      ;[1 1 1] Draught
      (Utilities|FlowControl|DoOnce false) ; enters at Reset
    )))

(event EventTick
  (params (DeltaSeconds :type Float%20%28single-precision%29))
  ;[1 1 1] Setting the weather and initiating the event
  (Utilities|FlowControl|Sequence
    (:then_0
      (Utilities|FlowControl|Delay 0.2)
      (switch Utilities|FlowControl|Switch|SwitchonEnum_WeatherStatus (Variables|Default|GetWeatherStatus)
        (:NewEnumerator0
          (CallFunction|Normal "Normal"))
        (:NewEnumerator1
          (CallFunction|Raining "Raining")
          (Variables|Default|SetHasRainStopped (<= (Variables|Default|GetRainAmount) 0.0) :!label _label)
          (Variables|Default|SetHasSnowStopped (<= (Variables|Default|GetSnowAmount) 0.0)))
        (:NewEnumerator2
          (CallFunction|Snowing "Snowing")
          (goto _label))
        (:NewEnumerator3
          (CallFunction|Draught "Draught"))))
    (:then_1
      (Utilities|FlowControl|Delay 3e+01)
      (Variables|Default|SetWeatherStatus (Utilities|Enum|ByteToEnumEnum_WeatherStatus (Math|Conversions|ToByte(Integer) (Math|Random|RandomIntegerinRange 0 (- (|GetNumEnumEntries) 1)))))
      (Utilities|FlowControl|Sequence
        (:then_0
          (Utilities|FlowControl|DoOnce false) ; enters at Reset
        )
        (:then_1
          ;[1 1 1] Normal
          (Utilities|FlowControl|DoOnce false) ; enters at Reset
        )
        (:then_2
          (Utilities|FlowControl|DoOnce false) ; enters at Reset
        )
        (:then_3
          ;[1 1 1] Draught
          (Utilities|FlowControl|DoOnce false) ; enters at Reset
        )))))

(fn ConstructionScript)